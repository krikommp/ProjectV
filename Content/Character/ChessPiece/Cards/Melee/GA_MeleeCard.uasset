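; GA_MeleeCard is the Gameplay Ability for a chess piece's melee card, applying a melee effect toward a chosen grid tile.
; Activation waits for card input, turns the piece to look at the target tile, then applies the physics melee effect container with range scaled by ability level.
; It then commits and ends after a short delay.
; A helper formats the level-based cost as display text.
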(event `self.K2_ActivateAbility`
  (bind (_asynctaskproxy _cardabilityinputevent) (`GridAbilityTask_WaitCardAbilityInputEvent.WaitCardAbilityInputEvent`)
    (:`OnGridAbilityInputEvent`
      (`GridAbilityTask_WaitChessPieceLookAt.WaitChessPieceLookAt` (`.TargetTileIndex` (break `GridAbilityInputEvent` _cardabilityinputevent))
        (:`OnWaitChessPieceLookAt`
          (`self.ApplyEffectContainer` (struct :`TagName` "CardAbility.Physics.Melee") (`.TargetTileIndex` (break `GridAbilityInputEvent` _cardabilityinputevent)) (`self.GetCardAbilityRange` (`self.GetAbilityLevel`)))
          (`self.K2_CommitAbility`)
          (`KismetSystemLibrary.Delay` 0.2)
          (`self.K2_EndAbility`))))))

(event `self.K2_OnEndAbility`
  (params (bWasCancelled :type Boolean)))

(fn `GetCardAbilityCostForDisplay`
  (params (InCardAbilityLevel :type Integer))
  (returns (ReturnValue :type Text))
  (return (`KismetTextLibrary.Conv_IntToText` (`self.GetCardAbilityCost` InCardAbilityLevel))))